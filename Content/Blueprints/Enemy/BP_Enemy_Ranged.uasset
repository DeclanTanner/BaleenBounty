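; Ranged enemy Blueprint that handles taking hits from the player and dying; no attack logic appears in its graphs.
; PlayerDealtDamage plays one of two random hit montages and subtracts fixed Health, rechecking it when the montage completes or is interrupted.
; At zero Health it disables capsule collision, ragdolls the mesh and destroys itself after a delay.
; The GettingHit guard clears before the montage plays, so hits can overlap.
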(event `/Game/Blueprints/Interface_OnAttackedByPlayer.PlayerDealtDamage`
  (params (AttackID :type Integer))
  (if (not (`self.GettingHit`))
    (set `self.GettingHit` true)
    (if (<= (`self.Health`) 0.0)
      (`PrimitiveComponent.SetCollisionEnabled` (`self.CapsuleComponent`) "NoCollision")
      (`PrimitiveComponent.SetCollisionEnabled` (`self.Mesh`) "QueryAndPhysics")
      (`PrimitiveComponent.SetSimulatePhysics` (`self.Mesh`) true)
      (`KismetSystemLibrary.Delay` 5.0)
      (`self.K2_DestroyActor` self)
      (else
        (set `self.GettingHit` false)
        (`|PlayMontage` (`self.Mesh`) (select `int` (`KismetMathLibrary.RandomIntegerInRange` 0 1) :`0` "/Game/ARPG_Warrior/Animations_UE5/ARPG_Warrior_Anim_UE_Hit4_Montage.ARPG_Warrior_Anim_UE_Hit4_Montage" :`1` "/Game/ARPG_Warrior/Animations_UE5/ARPG_Warrior_Anim_UE_Hit14_Montage.ARPG_Warrior_Anim_UE_Hit14_Montage" :!type "AnimMontage Object Reference") 1.5
          (:`then`
            (bind _output_get (set `self.Health` (- (`self.Health`) 50.0))))
          (:`OnCompleted`
            (if (<= (`self.Health`) 0.0) :!label _label
              (`PrimitiveComponent.SetCollisionEnabled` (`self.CapsuleComponent`) "NoCollision")
              (`PrimitiveComponent.SetCollisionEnabled` (`self.Mesh`) "QueryAndPhysics")
              (`PrimitiveComponent.SetSimulatePhysics` (`self.Mesh`) true)
              (`KismetSystemLibrary.Delay` 5.0)
              (`self.K2_DestroyActor` self)
              (else
                (set `self.GettingHit` false))))
          (:`OnInterrupted`
            (goto _label)))))))

(fn `UserConstructionScript`
  (`parent.UserConstructionScript`))