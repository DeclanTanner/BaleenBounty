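; Base enemy Blueprint for melee combat that punches the player, reacts to hits and ragdolls on death.
; Attack plays a random punch montage and fires OnAttackEnd when it ends.
; EnemyHitDetection sphere-traces pawns at the left-hand socket and sends damage to the hit actor.
; PlayerDealtDamage plays a hit montage and lowers Health, or, if Health is already depleted, launches the ragdoll away from the player before destroying it.
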(event `Attack`
  (`|PlayMontage` (`self.Mesh`) (select `int` (`KismetMathLibrary.RandomIntegerInRange` 0 1) :`0` "/Game/Animations/Player/AM_Player_Left_Punch.AM_Player_Left_Punch" :`1` "/Game/Animations/Player/AM_Player_Right_Punch.AM_Player_Right_Punch" :!type "AnimMontage Object Reference")
    (:`OnCompleted`
      _)
    (:`OnInterrupted`
      _))
  (`self.OnAttackEnd`))

(event `/Game/Blueprints/Interface_OnAttackedByPlayer.PlayerDealtDamage`
  (params (AttackID :type Integer))
  (if (not (`self.GettingHit`))
    (set `self.GettingHit` true)
    (if (<= (`self.Health`) 0.0)
      (`PrimitiveComponent.SetCollisionEnabled` (`self.CapsuleComponent`) "NoCollision")
      (`PrimitiveComponent.SetCollisionEnabled` (`self.Mesh`) "QueryAndPhysics")
      (`PrimitiveComponent.SetSimulatePhysics` (`self.Mesh`) true)
      (`PrimitiveComponent.AddImpulseAtLocation` (`self.Mesh`) (`KismetMathLibrary.MakeVector` (.x (* (`KismetMathLibrary.Normal` (- (`self.K2_GetActorLocation`) (`self.K2_GetActorLocation` (`GameplayStatics.GetPlayerCharacter` 0)))) (30000.0 30000.0 0.0))) (.y (* (`KismetMathLibrary.Normal` (- (`self.K2_GetActorLocation`) (`self.K2_GetActorLocation` (`GameplayStatics.GetPlayerCharacter` 0)))) (30000.0 30000.0 0.0)))) (0.0 0.0 0.0) "None")
      (`KismetSystemLibrary.Delay` 5.0)
      (`self.K2_DestroyActor` self)
      (else
        (set `self.GettingHit` false)
        (`|PlayMontage` (`self.Mesh`) (select `int` (`KismetMathLibrary.RandomIntegerInRange` 0 1) :`0` "/Game/ARPG_Warrior/Animations_UE5/ARPG_Warrior_Anim_UE_Hit4_Montage.ARPG_Warrior_Anim_UE_Hit4_Montage" :`1` "/Game/ARPG_Warrior/Animations_UE5/ARPG_Warrior_Anim_UE_Hit14_Montage.ARPG_Warrior_Anim_UE_Hit14_Montage" :!type "AnimMontage Object Reference") 1.5
          (:`then`
            (bind _output_get (set `self.Health` (- (`self.Health`) 50.0))))
          (:`OnCompleted`
            (if (not (<= (`self.Health`) 0.0)) :!label _label
              (set `self.GettingHit` false)))
          (:`OnInterrupted`
            (goto _label)))))))

(fn `EnemyHitDetection`
  (bind _returnvalue (`SceneComponent.GetSocketLocation` (`self.Mesh`) (select `int` 0 :`0` "hand_l" :`1` "hand_r" :!type "Name")))
  ;[1 1 1] Create attack hitbox, for each WorldDynamic object in the hitbox, send an attack command
  (bind _outhit (`KismetSystemLibrary.SphereTraceSingleForObjects` :`Start` _returnvalue :`End` _returnvalue :`Radius` 50.0 :`ObjectTypes` (`|MakeArray` "ObjectTypeQuery3" :!type "EObjectTypeQuery Enum") :`DrawDebugType` "ForDuration"))
  (message `/Game/Blueprints/Interface_OnPlayerHurt.PlayerReceivedDamage` (`.HitActor` (`GameplayStatics.BreakHitResult` _outhit)) 25.0))

(fn `UserConstructionScript`)