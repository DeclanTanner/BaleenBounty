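; Spawner actor that populates an area with randomly chosen enemies when the player pawn overlaps its Trigger, provided none of its previous spawns remain.
; It spawns AmountToSpawn actors from ClassesToSpawn at random XY points within the Location box, each yawed toward the player.
; Each spawn is tracked until destroyed; emptying the list fires OnEnemiesDefeated and lets the trigger spawn again.
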(event `self.Trigger.OnComponentBeginOverlap`
  (params (OverlappedComponent :type "PrimitiveComponent Object Reference") (OtherActor :type "Actor Object Reference") (OtherComp :type "PrimitiveComponent Object Reference") (OtherBodyIndex :type Integer) (bFromSweep :type Boolean) (SweepResult :type "HitResult Structure (by ref)"))
  (bind _location (`self.Location`))
  (bind (_returnvalue_x _returnvalue_y _returnvalue_z) (`KismetMathLibrary.BreakVector` (`SceneComponent.K2_GetComponentLocation` _location)))
  (bind (_boxextent_x _boxextent_y) (`KismetMathLibrary.BreakVector` (`BoxComponent.BoxExtent` _location)))
  (bind _returnvalue (`KismetMathLibrary.MakeVector` (`KismetMathLibrary.RandomFloatInRange` (- _returnvalue_x _boxextent_x) (+ _returnvalue_x _boxextent_x)) (`KismetMathLibrary.RandomFloatInRange` (- _returnvalue_y _boxextent_y) (+ _returnvalue_y _boxextent_y)) _returnvalue_z))
  (bind (_returnvalue_roll _returnvalue_pitch _returnvalue_yaw) (`KismetMathLibrary.BreakRotator` (`KismetMathLibrary.FindLookAtRotation` _returnvalue (`self.K2_GetActorLocation` (`GameplayStatics.GetPlayerPawn` 0)))))
  (if (and (== OtherActor (`GameplayStatics.GetPlayerPawn` 0)) (`KismetArrayLibrary.Array_IsEmpty` (`self.SpawnedActors`)))
    (for _ (range 1 (+ (`self.AmountToSpawn`) 1))
      (bind _returnvalue_2 (`|SpawnActorFromClass` (`KismetArrayLibrary.Array_Random` (`self.ClassesToSpawn`)) (`KismetMathLibrary.MakeTransform` _returnvalue (`KismetMathLibrary.MakeRotator` 0.0 0.0 _returnvalue_yaw)) "AlwaysSpawn" "MultiplyWithRoot" null null))
      (`/Engine/EditorBlueprintResources/StandardMacros.IsValid` _returnvalue_2
        (:`Is Valid`
          (add `self.OnDestroyed` _returnvalue_2 (delegate `OnDestroyed_Event`))
          (`KismetArrayLibrary.Array_Add` (`self.SpawnedActors`) _returnvalue_2))))))

(event `OnDestroyed_Event` :!signature `self.OnDestroyed`
  (params (DestroyedActor :type "Actor Object Reference"))
  (bind _spawnedactors (`self.SpawnedActors`))
  (`KismetArrayLibrary.Array_RemoveItem` _spawnedactors DestroyedActor)
  (if (`KismetArrayLibrary.Array_IsEmpty` _spawnedactors)
    (`self.OnEnemiesDefeated`)))

(fn `UserConstructionScript`)